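; Player character Blueprint that sets up the player's UI and handles the quit input.
; On BeginPlay it adds the HUD to the viewport, binds to OnPlayerRespawn and creates a world health bar widget attached to itself.
; Each respawn creates and displays a new health bar, replacing the stored reference without removing the previous widget here.
; The IA_QuitGame Enhanced Input action quits the game.
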(event `self.ReceiveBeginPlay`
  (bind _returnvalue (`|CreateWidget` "/Game/Core/UI/WBP_HUD.WBP_HUD_C"))
  (`UserWidget.AddToViewport` _returnvalue 0)
  (add `self.OnPlayerRespawn` (delegate `OnPlayerRespawn_Event`))
  (bind _returnvalue_2 (`|CreateWidget` "/Game/Core/UI/PlayerStats/WBP_WorldHealthBar.WBP_WorldHealthBar_C" null self))
  (bind _output_get (set `self.WorldHealthBarWidget` _returnvalue_2))
  (`UserWidget.AddToViewport` _output_get 0))

(event `OnPlayerRespawn_Event`
  (bind _returnvalue (`|CreateWidget` "/Game/Core/UI/PlayerStats/WBP_WorldHealthBar.WBP_WorldHealthBar_C" null self))
  (bind _output_get (set `self.WorldHealthBarWidget` _returnvalue))
  (`UserWidget.AddToViewport` _output_get 0))

(event `EnhancedInput|/Game/Core/Input/InputActions/IA_QuitGame`
  (params (ActionValue :type Boolean) (ElapsedSeconds :type "Float (double-precision)") (TriggeredSeconds :type "Float (double-precision)") (InputAction :type "InputAction Object Reference" :default "/Game/Core/Input/InputActions/IA_QuitGame.IA_QuitGame"))
  (:`Started`
    (`KismetSystemLibrary.QuitGame` null "Quit")))

(fn `UserConstructionScript`)